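; BP_Pawn is a player camera pawn with pan, zoom and stepped yaw rotation controls.
; Input events update desired location, clamped spring arm length and rotation, with panning relative to the actor's forward and right vectors and each rotation press adding a fixed yaw step.
; Tick eases the actor transform and arm length toward those targets with separate interpolation speeds, moving without sweep collision.
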(event `self.ReceiveBeginPlay`
  ;[0.4375 0.4526 1] set (location_desired, zoom_desired, rotation_desired) at start
  (set `self.Location_Desired` (`self.K2_GetActorLocation`))
  (set `self.Zoom_Desired` (`SpringArmComponent.TargetArmLength` (`self.SpringArm`)))
  (set `self.Rotation_Desired` (`self.K2_GetActorRotation`)))

(event `self.ReceiveTick`
  (params (DeltaSeconds :type "Float (single-precision)"))
  (bind _springarm (`self.SpringArm`))
  ;[0.1779 0.1845 0.4072] interpolate camera zoom, camera location, camera rotation after movement
  (set `SpringArmComponent.TargetArmLength` (`KismetMathLibrary.FInterpTo` (`SpringArmComponent.TargetArmLength` _springarm) (`self.Zoom_Desired`) DeltaSeconds (`self.Zoom_Interp`)) _springarm)
  (`self.K2_SetActorLocation` (`KismetMathLibrary.VInterpTo` (`self.K2_GetActorLocation`) (`self.Location_Desired`) DeltaSeconds (`self.Location_Interp`)))
  (`self.K2_SetActorRotation` (`KismetMathLibrary.RInterpTo` (`self.K2_GetActorRotation`) (`self.Rotation_Desired`) DeltaSeconds (`self.Rotation_Interp`))))

(event `InputAxis|InputAxis_Zoom`
  (params (AxisValue :type "Float (single-precision)"))
  ;[1 1 1] camera zoom controls
  (set `self.Zoom_Desired` (`KismetMathLibrary.FClamp` (+ (`self.Zoom_Desired`) (* AxisValue (`self.Zoom_Speed`))) (`self.Zoom_Min`) (`self.Zoom_Max`))))

(event `InputAxis|InputAxis_Forward`
  (params (AxisValue :type "Float (single-precision)"))
  ;[1 1 1] camera movement controls
  (set `self.Location_Desired` (+ (`self.Location_Desired`) (* (`self.GetActorForwardVector`) (* AxisValue (`self.Location_Speed`))))))

(event `InputAxis|InputAxis_Right`
  (params (AxisValue :type "Float (single-precision)"))
  ;[1 1 1] camera movement controls
  (set `self.Location_Desired` (+ (`self.Location_Desired`) (* (`self.GetActorRightVector`) (* AxisValue (`self.Location_Speed`))))))

(event `InputAction|InputAction_RotationRight`
  (params (Key :type "Key Structure"))
  ;[1 1 1] camera rotation controls
  (:`Pressed`
    (set `self.Rotation_Desired` (`KismetMathLibrary.ComposeRotators` (`self.Rotation_Desired`) (`KismetMathLibrary.MakeRotator` 0.0 0.0 (- 0.0 (`self.Rotation_Speed`)))))))

(event `InputAction|InputAction_rotationLeft`
  (params (Key :type "Key Structure"))
  ;[1 1 1] camera rotation controls
  (:`Pressed`
    (set `self.Rotation_Desired` (`KismetMathLibrary.ComposeRotators` (`self.Rotation_Desired`) (`KismetMathLibrary.MakeRotator` 0.0 0.0 (`self.Rotation_Speed`))))))

(fn `UserConstructionScript`)