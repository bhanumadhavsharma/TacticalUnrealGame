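; BP_Grid builds a tile grid of hexagons, squares or triangles as instanced static meshes around a center location.
; SpawnGrid clears old instances, loads mesh and material from DT_GridShapeData, snaps the center, then places tiles from the bottom-left corner with per-shape spacing.
; Hexagons use staggered indices and triangles alternate yaw.
; Optional sphere traces snap tile height to ground and skip misses; the construction script's SpawnGrid call is disconnected.
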(fn `CalculateCenterAndBottomLeft`
  (returns (Center :type "Vector Structure") (BottomLeft :type "Vector Structure"))
  (locals (C :type "Vector Structure" :default (0.0 0.0 0.0)))
  (bind (_grid_tile_count_x _grid_tile_count_y) (break `IntPoint` (`self.Grid Tile Count`)))
  (switch `/Game/Blueprints/Core/Grid/GridShapes/Enum_GridShape` (`self.Grid Shape`)
    (:`NewEnumerator1`
      ;[1 1 1] hexagon
      (bind _output_get (set `local.C` (`/Game/Blueprints/Core/Utilities/BFL_Utilities.SnapVectorToVector` (`self.Grid Center Location`) (* (`self.Grid Tile Size`) (1.5 1.0 1.0)))))
      (return _output_get (- _output_get (`/Game/Blueprints/Core/Utilities/BFL_Utilities.SnapVectorToVector` (`KismetMathLibrary.Conv_Vector2DToVector` (* (/ (`KismetMathLibrary.Conv_IntPointToVector2D` (`self.Grid Tile Count`)) (3.0 2.0)) (`KismetMathLibrary.Conv_VectorToVector2D` (`self.Grid Tile Size`)))) (* (`self.Grid Tile Size`) (1.5 1.0 1.0))))))
    (:`NewEnumerator2`
      ;[1 1 1] square
      (bind _output_get_2 (set `local.C` (`/Game/Blueprints/Core/Utilities/BFL_Utilities.SnapVectorToVector` (`self.Grid Center Location`) (`self.Grid Tile Size`))))
      (return _output_get_2 (- _output_get_2 (`KismetMathLibrary.Conv_Vector2DToVector` (* (/ (- (`KismetMathLibrary.Conv_IntPointToVector2D` (`self.Grid Tile Count`)) (`KismetMathLibrary.MakeVector2D` (`KismetMathLibrary.SelectFloat` 0.0 1.0 (`/Game/Blueprints/Core/Utilities/BFL_Utilities.IsIntEven` _grid_tile_count_x)) (`KismetMathLibrary.SelectFloat` 0.0 1.0 (`/Game/Blueprints/Core/Utilities/BFL_Utilities.IsIntEven` _grid_tile_count_y)))) 2.0) (`KismetMathLibrary.Conv_VectorToVector2D` (`self.Grid Tile Size`)))))))
    (:`NewEnumerator3`
      ;[1 1 1] triangle
      (bind _output_get_3 (set `local.C` (`/Game/Blueprints/Core/Utilities/BFL_Utilities.SnapVectorToVector` (`self.Grid Center Location`) (* (`self.Grid Tile Size`) (2.0 1.0 1.0)))))
      (return _output_get_3 (- _output_get_3 (`/Game/Blueprints/Core/Utilities/BFL_Utilities.SnapVectorToVector` (`KismetMathLibrary.Conv_Vector2DToVector` (* (/ (- (`KismetMathLibrary.Conv_IntPointToVector2D` (`self.Grid Tile Count`)) (-1.0 -1.0)) (2.0 4.0)) (`KismetMathLibrary.Conv_VectorToVector2D` (`self.Grid Tile Size`)))) (* (`self.Grid Tile Size`) (2.0 0.5 1.0))))))))

(fn `DestroyGrid`
  ;[1 1 1] delete all tile mesh instances
  (`InstancedStaticMeshComponent.ClearInstances` (`self.InstancedStaticMesh`)))

(fn `GetCurrentShapeData`
  (returns (ReturnValue :type "/Game/Blueprints/Core/Grid/GridShapes/F_GridShapeData Structure"))
  (bind _returnvalue (`|GetEnumeratorNameAsString` (`self.Grid Shape`)))
  (bind _returnvalue_2 (`|GetDataTableRow` "/Game/Blueprints/Core/Grid/GridShapes/DT_GridShapeData.DT_GridShapeData" (`KismetStringLibrary.Conv_StringToName` _returnvalue))
    (:`then`
      (return _returnvalue_2))
    (:`RowNotFound`
      (`KismetSystemLibrary.PrintString` (`KismetStringLibrary.Concat_StrStr` "Error - Row Not Found: " _returnvalue) true true (struct :`R` 1.0 :`G` 0.009844 :`A` 1.0) 5.0))))

(fn `GetTileLocationFromGridIndex`
  (params (GridIndex :type "IntPoint Structure"))
  (returns (TileLocation :type "Vector Structure"))
  (return (+ (`self.GridBottomLeftCornerLocation`) (* (`self.Grid Tile Size`) (`KismetMathLibrary.Conv_Vector2DToVector` (* (`KismetMathLibrary.Conv_IntPointToVector2D` GridIndex) (select `/Game/Blueprints/Core/Grid/GridShapes/Enum_GridShape` (`self.Grid Shape`) :`NewEnumerator1` (0.75 0.5) :`NewEnumerator2` (1.0 1.0) :`NewEnumerator3` (1.0 0.5) :!type "Vector2D Structure")))))))

(fn `GetTileRotationFromGridIndex`
  (params (GridIndex :type "IntPoint Structure"))
  (returns (TileRotation :type "Rotator Structure"))
  (if (`|EnumEquality` (`self.Grid Shape`) "NewEnumerator3")
    (return (`KismetMathLibrary.MakeRotator` 0.0 0.0 (+ (`KismetMathLibrary.SelectFloat` 180.0 0.0 (`/Game/Blueprints/Core/Utilities/BFL_Utilities.IsIntEven` GridIndex_X)) (`KismetMathLibrary.SelectFloat` 180.0 0.0 (`/Game/Blueprints/Core/Utilities/BFL_Utilities.IsIntEven` GridIndex_Y)))))
    (else
      (return))))

(fn `SetGridOffsetFromGround`
  (params (Offset :type "Float (double-precision)"))
  (bind _output_get (set `self.GridOffsetFromGround` Offset))
  (`SceneComponent.K2_SetWorldLocation` (`self.InstancedStaticMesh`) (`KismetMathLibrary.MakeVector` 0.0 0.0 _output_get) false false))

(fn `SpawnGrid`
  (params (CenterLocation :type "Vector Structure") (TileSize :type "Vector Structure") (TileCount :type "IntPoint Structure") (Shape :type "/Game/Blueprints/Core/Grid/GridShapes/Enum_GridShape Enum" :default "NewEnumerator0") (UseEnvironment :type Boolean))
  (locals (xIndex :type Integer) (yIndex :type Integer) (TileTransform :type "Transform Structure") (Index :type "IntPoint Structure"))
  (bind _instancedstaticmesh (`self.InstancedStaticMesh`))
  (bind (_tiletransform_location _tiletransform_rotation _tiletransform_scale) (`KismetMathLibrary.BreakTransform` (`local.TileTransform`)))
  (bind (_grid_tile_count_x _grid_tile_count_y) (break `IntPoint` (`self.Grid Tile Count`)))
  (bind _index (`local.Index`))
  (bind (_grid_tile_count_x_2 _grid_tile_count_y_2) (break `IntPoint` (`self.Grid Tile Count`)))
  (bind _grid_tile_count_x_3 (break `IntPoint` (`self.Grid Tile Count`)))
  (bind (_meshsize _mesh _meshmaterial _flatmesh _flatmesh_bordermaterial) (break `/Game/Blueprints/Core/Grid/GridShapes/F_GridShapeData` (`self.GetCurrentShapeData`)))
  ;[1 1 1] set variables
  (set `self.Grid Center Location` CenterLocation)
  (set `self.Grid Tile Size` TileSize)
  (set `self.Grid Shape` Shape)
  (set `self.Grid Tile Count` TileCount)
  (`self.DestroyGrid`)
  ;[1 1 1] get shape
  (`StaticMeshComponent.SetStaticMesh` _instancedstaticmesh _flatmesh)
  (`PrimitiveComponent.SetMaterial` _instancedstaticmesh 0 _flatmesh_bordermaterial)
  (`self.SetGridOffsetFromGround` (`self.GridOffsetFromGround`))
  ;[0.5573 0.2932 0.2932] spawn tiles:
  ; 1) get bottom left corner locatin using the center spot, and its distance from corner spot
  ; 2) get x and y of every shape from bottom left corner (effectively just get the coordinates of every shape starting from 0,0 -> 0,1 -> 0,n -> 1,0 -> 1,1 -> 1,n -> 2,0 ->...)
  ; 3) set shape correctly (ex. if triangle, it must be up then down, then up, then down)
  ; 4.1) start setting down the shapes from bottom left (set their transform using the data we've collected)
  ; 4.2) create the instance
  ;;[1 1 1] 1) get bottom left corner locatin using the center spot, and its distance from corner spot
  (bind (_center _bottomleft) (`self.CalculateCenterAndBottomLeft`))
  (set `self.Grid Center Location` _center)
  (set `self.GridBottomLeftCornerLocation` _bottomleft)
  ;;[1 1 1] 2) get x and y of every shape from bottom left corner (effectively just get the coordinates of every shape starting from 0,0 -> 0,1 -> 0,n -> 1,0 -> 1,1 -> 1,n -> 2,0 ->...)
  (for _index_2 (range _grid_tile_count_x_3)
    (set `local.xIndex` _index_2)
    ;;;[1 1 1] check if not hexagon
    (if (`|EnumInequality` (`self.Grid Shape`) "NewEnumerator1")
      ;;;[1 1 1] y index for triangles and squares
      (for _index_3 (range _grid_tile_count_y)
        (set `local.yIndex` _index_3)
        ;;[1 1 1] 2.1) set x and y indexes as one variable
        (set `local.Index` (make `IntPoint` (`local.xIndex`) (`local.yIndex`)) :!label _label)
        ;;[1 1 1] 4.1) start setting down the shapes from bottom left (set their transform using the data we've collected)
        ;; 4.2) create the instance
        (set `local.TileTransform` (`KismetMathLibrary.MakeTransform` (`self.GetTileLocationFromGridIndex` _index) (`self.GetTileRotationFromGridIndex` _index) (/ (`self.Grid Tile Size`) (`.MeshSize_2_846AFC5F4BCBE774F56AAD96A69108BD` (break `/Game/Blueprints/Core/Grid/GridShapes/F_GridShapeData` (`self.GetCurrentShapeData`))))))
        (if (`local.UseEnvironment`)
          ;[1 1 1] trace to see ground
          (bind (_hitsomething _outlocation) (`self.TraceForGround` _tiletransform_location))
          (if _hitsomething
            (set `local.TileTransform` (`KismetMathLibrary.MakeTransform` _outlocation _tiletransform_rotation _tiletransform_scale))
            ;[1 1 1] Spawn Tile Mesh
            (`InstancedStaticMeshComponent.AddInstance` (`self.InstancedStaticMesh`) (`local.TileTransform`)))
          (else
            ;[1 1 1] Spawn Tile Mesh
            (`InstancedStaticMeshComponent.AddInstance` (`self.InstancedStaticMesh`) (`local.TileTransform`)))))
      (else
        ;;;[1 1 1] y index for hexagons
        (for _index_4 (range (`KismetMathLibrary.SelectInt` 0 1 (`/Game/Blueprints/Core/Utilities/BFL_Utilities.IsIntEven` (`local.xIndex`))) (* _grid_tile_count_y_2 2))
          (set `local.yIndex` _index_4)
          (`|ExecutionSequence`
            (:`then_0`
              (goto _label))
            (:`then_1`
              (`/Engine/EditorBlueprintResources/StandardMacros.IncrementInt` _index_4))))))))

(fn `TraceForGround`
  (params (TileLocation :type "Vector Structure"))
  (returns (HitSomething :type Boolean) (OutLocation :type "Vector Structure"))
  (locals (Radius :type "Float (double-precision)" :default 0.0))
  (bind _tilelocation (`local.TileLocation`))
  (bind _grid_tile_size_x (`KismetMathLibrary.BreakVector` (`self.Grid Tile Size`)))
  (bind (_tilelocation_x _tilelocation_y) (`KismetMathLibrary.BreakVector` (`local.TileLocation`)))
  (bind (_grid_tile_size_x_2 _grid_tile_size_y _grid_tile_size_z) (`KismetMathLibrary.BreakVector` (`self.Grid Tile Size`)))
  (set `local.Radius` (/ _grid_tile_size_x (`KismetMathLibrary.SelectFloat` 5.0 3.0 (`|EnumEquality` (`self.Grid Shape`) "NewEnumerator3"))))
  (bind _outhits (`KismetSystemLibrary.SphereTraceMulti` (+ _tilelocation (0.0 0.0 1000.0)) (- _tilelocation (0.0 0.0 1000.0)) (`local.Radius`) "TraceTypeQuery3"))
  (if (> (`KismetArrayLibrary.Array_Length` _outhits) 0)
    (return true (`KismetMathLibrary.MakeVector` _tilelocation_x _tilelocation_y (`KismetMathLibrary.GridSnap_Float` (- (.z (`.Location` (`GameplayStatics.BreakHitResult` (`|GetArrayItem` _outhits)))) (`local.Radius`)) _grid_tile_size_z)))
    (else
      (return false (`local.TileLocation`)))))

(fn `UserConstructionScript`)